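; Chat game mode that runs a turn-based number baseball game, relaying messages and results to all BP_ChatPlayerControllers.
; Judges commands against three random numbers, rejecting consecutive guesses from the same player and decrementing the sender's remaining attempts.
; A looping turn timer, restarted on guesses, charges an attempt to a player other than the last mover and passes the turn.
; A win updates scores and resets the game; all players running out declares a draw.
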(event Custom|MessagefromJudge_Event
  (params (UserID :type String) (Message :type String) (Sender :type BP%20Chat%20Player%20Controller%20Object%20Reference))
  ;[0.15 0.15 0.15 0.5] 채팅 입력이 명령어인 경우
  (Variables|Default|SetSender Sender)
  (bind _returnvalue (Class|NumberBaseballLib|IsGameCommand Message))
  (if _returnvalue
    (bind _bisturninprogress (CallFunction|TurnCheck UserID))
    (if _bisturninprogress
      (Utilities|FlowControl|Sequence
        (:then_0
          ;;[0.15 0.15 0.15 0.5] 숫자 야구 시도 횟수가 남았는지 확인 및 처리
          (if (> (Variables|/Game/Blueprints/BP_ChatPlayerController.BP_ChatPlayerController_C|GetRemainInputCount (Variables|Default|GetSender)) 0)
            ;;[0.15 0.15 0.15 0.5] 남은 명령어 횟수 감소 및 출력
            (CallFunction|DecreaseRemainInput (Variables|Default|GetSender))
            ;;[0.15 0.15 0.15 0.5] 기존 타이머 초기화 및 새로운 타이머 설정
            (Utilities|Time|ClearTimerbyFunctionName 0 "OnTurnTimeExpired")
            (Utilities|Time|SetTimerbyFunctionName 0 "OnTurnTimeExpired" (Variables|Default|GetTurnTime) true)))
        (:then_1
          (if (> (Variables|/Game/Blueprints/BP_ChatPlayerController.BP_ChatPlayerController_C|GetRemainInputCount (Variables|Default|GetSender)) 0)
            ;;[0.15 0.15 0.15 0.5] 플레이어의 입력을 확인하고 판정 처리
            (bind (_strikes _balls _returnvalue_2) (Class|NumberBaseballLib|JudgeNumber (Variables|Default|GetbaseballNumber) Message))
            (Utilities|FlowControl|Sequence
              (:then_0
                (CallFunction|AllPlayerCallBroadcastEvent _returnvalue_2))
              (:then_1
                (bind _returnvalue_3 (Class|NumberBaseballLib|HasPlayerWon _strikes _balls))
                (if _returnvalue_3
                  (CallFunction|AllPlayerCallBroadcastEvent (Utilities|String|Append UserID "승리!"))
                  (CallFunction|ResetGame)
                  (bind _outactors (Actor|GetAllActorsOfClass "/Script/Engine.PlayerController"))
                  (for _array_element _outactors
                    (bind _asbp_chat_player_controller (Utilities|Casting|CastToBP_ChatPlayerController _array_element))
                    (Default|OnChangeScore _asbp_chat_player_controller (Variables|/Game/Blueprints/BP_ChatPlayerController.BP_ChatPlayerController_C|GetUserID (Variables|Default|GetSender)))))))))
        (:then_2
          ;;[0.15 0.15 0.15 0.5] 남은 기회에 대한 판정 및 출력
          (CallFunction|EvaluateRemainingInput (Variables|Default|GetSender)))))))

(event Custom|MessagefromClient_Event
  (params (Message :type String))
  ;[0.15 0.15 0.15 0.5] 모든 플레이어에게 채팅 전달
  (CallFunction|AllPlayerCallBroadcastEvent Message))

(event EventBeginPlay
  ;[0.15 0.15 0.15 0.5] 게임 시작시 숫자 3개 랜덤으로 설정
  (Variables|Default|SetbaseballNumber (Class|NumberBaseballLib|GenerateRandomNumbers))
  (Variables|Default|SetTurnTime 1e+01))

(fn ConstructionScript)

(fn DecreaseRemainInput
  (params (TargetPlayerController :type BP%20Chat%20Player%20Controller%20Object%20Reference))
  ;[0.15 0.15 0.15 0.5] 플레이어의 남은 횟수 감소 및 출력
  (bind _result (Math|Integer|DecrementInt (Variables|/Game/Blueprints/BP_ChatPlayerController.BP_ChatPlayerController_C|GetRemainInputCount TargetPlayerController))
    (:%20%20
      (bind _output_get (Variables|/Game/Blueprints/BP_ChatPlayerController.BP_ChatPlayerController_C|SetRemainInputCount TargetPlayerController _result))
      (CallFunction|AllPlayerCallBroadcastEvent (Utilities|String|ToString(Text) (Utilities|Text|FormatText "남은 입력 횟수: {Remain Input Count}" _output_get))))))

(fn TurnCheck
  (params (InputPlayerID :type String))
  ;[0.15 0.15 0.15 0.5] 이전에 진행한 플레이어와 같은지 확인
  (if (Utilities|Enum|NotEqual(Enum) (Variables|Default|GetPrevInputPlayerID) InputPlayerID)
    ;[0.15 0.15 0.15 0.5] 다른 경우
    (Variables|Default|SetPrevInputPlayerID InputPlayerID)
    (return true)
    (else
      ;[0.15 0.15 0.15 0.5] 같은 경우
      (CallFunction|AllPlayerCallBroadcastEvent (Utilities|String|ToString(Text) (Utilities|Text|FormatText "{ A }의 턴이 아닙니다." InputPlayerID)))
      (return false))))

(fn ResetGame
  ;[0.15 0.15 0.15 0.5] 게임을 초기화하는 로직
  (Utilities|FlowControl|Sequence
    (:then_0
      ;;[0.15 0.15 0.15 0.5] 출력
      (CallFunction|AllPlayerCallBroadcastEvent "게임을 초기화 합니다."))
    (:then_1
      ;;[0.15 0.15 0.15 0.5] 게임모드 변수 초기화
      (Variables|Default|SetbaseballNumber (Class|NumberBaseballLib|GenerateRandomNumbers))
      (Utilities|Time|ClearTimerbyFunctionName 0 "OnTurnTimeExpired")
      (Variables|Default|SetPrevInputPlayerID ""))
    (:then_2
      ;;[0.15 0.15 0.15 0.5] 플레이어 컨트롤러 변수 초기화
      (bind _outactors (Actor|GetAllActorsOfClass "/Script/Engine.PlayerController"))
      (for _array_element _outactors
        (bind _asbp_chat_player_controller (Utilities|Casting|CastToBP_ChatPlayerController _array_element))
        (Variables|/Game/Blueprints/BP_ChatPlayerController.BP_ChatPlayerController_C|SetRemainInputCount _asbp_chat_player_controller (Variables|/Game/Blueprints/BP_ChatPlayerController.BP_ChatPlayerController_C|GetMaxInputCount _asbp_chat_player_controller))))))

(fn AllPlayerCallBroadcastEvent
  (params (Massege :type String))
  ;[0.15 0.15 0.15 0.5] 모든 플레이어에게 메세지 전달
  (bind _outactors (Actor|GetAllActorsOfClass "/Script/Engine.PlayerController"))
  (for _array_element _outactors
    (bind _asbp_chat_player_controller (Utilities|Casting|CastToBP_ChatPlayerController _array_element))
    (Default|BroadcastEvent _asbp_chat_player_controller Massege)))

(fn OnTurnTimeExpired
  (Utilities|FlowControl|Sequence
    (:then_0
      ;[0.15 0.15 0.15 0.5] 출력
      (CallFunction|AllPlayerCallBroadcastEvent "시간 내에 입력하지 않아 기회가 소진됐습니다."))
    (:then_1
      ;[0.15 0.15 0.15 0.5] 입력 해야했던 플레이어를 찾는 로직
      (bind _outactors (Actor|GetAllActorsOfClass "/Script/Engine.PlayerController"))
      (for _array_element _outactors
        (bind _asbp_chat_player_controller (Utilities|Casting|CastToBP_ChatPlayerController _array_element))
        (if (Utilities|Enum|NotEqual(Enum) (Variables|/Game/Blueprints/BP_ChatPlayerController.BP_ChatPlayerController_C|GetUserID _asbp_chat_player_controller) (Variables|Default|GetPrevInputPlayerID))
          (Variables|Default|SetSender _asbp_chat_player_controller))))
    (:then_2
      ;[0.15 0.15 0.15 0.5] 플레이어 횟수 감소 및 무승부 확인
      (CallFunction|DecreaseRemainInput (Variables|Default|GetSender))
      (CallFunction|EvaluateRemainingInput (Variables|Default|GetSender)))
    (:then_3
      ;[0.15 0.15 0.15 0.5] 턴을 진행해야할 플레이어 변경
      (Variables|Default|SetPrevInputPlayerID (Variables|/Game/Blueprints/BP_ChatPlayerController.BP_ChatPlayerController_C|GetUserID (Variables|Default|GetSender))))))

(fn EvaluateRemainingInput
  (params (TargetPlayerController :type BP%20Chat%20Player%20Controller%20Object%20Reference))
  ;[0.15 0.15 0.15 0.5] 출력 및 무승부 확인
  (if (<= (Variables|/Game/Blueprints/BP_ChatPlayerController.BP_ChatPlayerController_C|GetRemainInputCount TargetPlayerController) 0)
    (CallFunction|AllPlayerCallBroadcastEvent "더 이상 기회가 없습니다.")
    (bind _outactors (Actor|GetAllActorsOfClass "/Script/Engine.PlayerController"))
    (for _array_element _outactors
      (bind _asbp_chat_player_controller (Utilities|Casting|CastToBP_ChatPlayerController _array_element))
      (if (>= 0 (Variables|/Game/Blueprints/BP_ChatPlayerController.BP_ChatPlayerController_C|GetRemainInputCount _asbp_chat_player_controller))
        (bind _output_get (Variables|Default|SetPlayersRemainInput (+ (Variables|Default|GetPlayersRemainInput) 1)))
        (if (>= _output_get (Utilities|Array|Length _outactors))
          (CallFunction|AllPlayerCallBroadcastEvent "모든 플레이어의 기회가 소진되어 무승부입니다.")
          (CallFunction|ResetGame))))))